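; Camera actor for a two-player fighting game that keeps both fighters framed.
; On BeginPlay, after a short delay, it caches both player references from FightingGamemodeBlueprint.
; Each Tick it moves to the players' midpoint in X and Z, keeping its Y and clamping X to gamemode limits.
; It widens or narrows field of view within a clamped range based on their horizontal separation relative to MaxDistance.
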(event EventBeginPlay
  (Utilities|FlowControl|Delay 0.2)
  (bind _asfighting_gamemode_blueprint (Utilities|Casting|CastToFightingGamemodeBlueprint (Game|GetGameMode)))
  (Variables|Default|SetgamemodeReference _asfighting_gamemode_blueprint)
  (Variables|Default|Setplayer1CameraReference (Variables|/Game/Gamemodes/FightingGamemodeBlueprint.FightingGamemodeBlueprint_C|Getplayer1Reference (Variables|Default|GetgamemodeReference)))
  (Variables|Default|Setplayer2CameraReference (Variables|/Game/Gamemodes/FightingGamemodeBlueprint.FightingGamemodeBlueprint_C|Getplayer2Reference (Variables|Default|GetgamemodeReference))))

(event Collision|EventActorBeginOverlap
  (params (OtherActor :type Actor%20Object%20Reference)))

(event EventTick
  (params (DeltaSeconds :type Float%20%28single-precision%29))
  (bind _player1camerareference (Variables|Default|Getplayer1CameraReference))
  (bind _gamemodereference (Variables|Default|GetgamemodeReference))
  (bind _player2camerareference (Variables|Default|Getplayer2CameraReference))
  (bind _returnvalue (Transformation|GetActorLocation _player2camerareference))
  (bind _returnvalue_2 (Transformation|GetActorLocation _player1camerareference))
  (Utilities|IsValid (Variables|Default|Getplayer1CameraReference)
    (:Is%20Valid
      (Utilities|IsValid (Variables|Default|Getplayer2CameraReference)
        (:Is%20Valid
          (Transformation|SetActorLocation (Math|Vector|MakeVector (Math|Float|Clamp(Float) (/ (+ (.x _returnvalue_2) (.x _returnvalue)) 2.0) (Variables|/Game/Gamemodes/FightingGamemodeBlueprint.FightingGamemodeBlueprint_C|GetminCameraX _gamemodereference) (Variables|/Game/Gamemodes/FightingGamemodeBlueprint.FightingGamemodeBlueprint_C|GetmaxCameraX _gamemodereference)) (.y (Transformation|GetActorLocation self)) (/ (+ (.z _returnvalue_2) (.z _returnvalue)) 2.0)) false false)
          (Camera|SetFieldOfView (Variables|Default|GetCameraComponent) (Math|Float|Clamp(Float) (+ (* (/ (Math|Float|Absolute(Float) (- (.x _returnvalue_2) (.x _returnvalue))) (Variables|/Script/ProjectW.MeshPlayerCharacter|GetmaxDistance (Variables|Default|Getplayer1CameraReference))) 3e+01) 9e+01) 1e+02 1.1e+02)))))))

(fn ConstructionScript)