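; Fighting-game box actor that serves as a proximity, strike or hurtbox for its owning player.
; SpawnHitbox sets the type's material, places and scales the hidden display at an offset mirrored by owner X facing, attaches to the owner, then checks collision once.
; CheckCollision finds the opponent through the game mode and tests overlap with their Hurtbox.
; Proximity overlaps notify the opponent; strikes set hitstun and blockstun frames and apply damage.
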(event Custom|SpawnHitbox
  (switch Utilities|FlowControl|Switch|SwitchonEHitboxType (Variables|Default|GethitboxType)
    (:PROXIMITY
      (Rendering|Material|SetMaterial (Variables|Default|GetHitboxDisplay) 0 "/Game/Materials/MProximityHitbox.MProximityHitbox"))
    (:STRIKE
      (Rendering|Material|SetMaterial (Variables|Default|GetHitboxDisplay) 0 "/Game/Materials/MStrikeHitbox.MStrikeHitbox"))
    (:HURTBOX
      (Rendering|Material|SetMaterial (Variables|Default|GetHitboxDisplay) 0 "/Game/Materials/MHurtboxHitbox.MHurtboxHitbox")))
  (bind _newhitboxlocation (CallFunction|GetNewHitboxLocation self))
  (Transformation|SetWorldLocation (Variables|Default|GetHitboxDisplay) _newhitboxlocation false false)
  (Transformation|SetWorldScale3D (Variables|Default|GetHitboxDisplay) (Variables|Default|GethitboxScale))
  (Rendering|SetVisibility (Variables|Default|GetHitboxDisplay) false false)
  (Transformation|AttachActorToActor (Components|GetOwner self) "None" "SnapToTarget" "SnapToTarget" "SnapToTarget" true)
  (CallFunction|CheckCollision))

(event Custom|CheckCollision
  (bind _asfighting_gamemode_blueprint (Utilities|Casting|CastToFightingGamemodeBlueprint (Game|GetGameMode)))
  (if (!= (Components|GetOwner self) (Variables|/Game/Gamemodes/FightingGamemodeBlueprint.FightingGamemodeBlueprint_C|Getplayer2Reference _asfighting_gamemode_blueprint))
    (if (Collision|IsOverlappingActor (Variables|/Game/Blueprints/Actors/MeshPlayerCharacterBlueprint.MeshPlayerCharacterBlueprint_C|Gethurtbox (Variables|/Game/Gamemodes/FightingGamemodeBlueprint.FightingGamemodeBlueprint_C|Getplayer2Reference _asfighting_gamemode_blueprint)) :!class /Script/Engine.Actor)
      (switch Utilities|FlowControl|Switch|SwitchonEHitboxType (Variables|Default|GethitboxType)
        (:PROXIMITY
          (Class|MeshPlayerCharacter|CollidedwithProximityHitbox (Variables|/Game/Gamemodes/FightingGamemodeBlueprint.FightingGamemodeBlueprint_C|Getplayer2Reference _asfighting_gamemode_blueprint)))
        (:STRIKE
          (Variables|/Script/ProjectW.MeshPlayerCharacter|SetcurrentHitstunFrames (Variables|/Game/Gamemodes/FightingGamemodeBlueprint.FightingGamemodeBlueprint_C|Getplayer2Reference _asfighting_gamemode_blueprint) (Variables|Default|GethitboxHitstunFrames))
          (Variables|/Script/ProjectW.MeshPlayerCharacter|SetcurrentBlockstunFrames (Variables|/Game/Gamemodes/FightingGamemodeBlueprint.FightingGamemodeBlueprint_C|Getplayer2Reference _asfighting_gamemode_blueprint) (Variables|Default|GethitboxBlockstunFrames))
          (Game|Damage|ApplyDamage (Variables|/Game/Gamemodes/FightingGamemodeBlueprint.FightingGamemodeBlueprint_C|Getplayer2Reference _asfighting_gamemode_blueprint) (Variables|Default|GethitboxDamage) 0 0))))
    (elif (Collision|IsOverlappingActor (Variables|/Game/Blueprints/Actors/MeshPlayerCharacterBlueprint.MeshPlayerCharacterBlueprint_C|Gethurtbox (Variables|/Game/Gamemodes/FightingGamemodeBlueprint.FightingGamemodeBlueprint_C|Getplayer1Reference _asfighting_gamemode_blueprint)) :!class /Script/Engine.Actor)
      (switch Utilities|FlowControl|Switch|SwitchonEHitboxType (Variables|Default|GethitboxType)
        (:PROXIMITY
          (Class|MeshPlayerCharacter|CollidedwithProximityHitbox (Variables|/Game/Gamemodes/FightingGamemodeBlueprint.FightingGamemodeBlueprint_C|Getplayer1Reference _asfighting_gamemode_blueprint)))
        (:STRIKE
          (Variables|/Script/ProjectW.MeshPlayerCharacter|SetcurrentHitstunFrames (Variables|/Game/Gamemodes/FightingGamemodeBlueprint.FightingGamemodeBlueprint_C|Getplayer1Reference _asfighting_gamemode_blueprint) (Variables|Default|GethitboxHitstunFrames))
          (Variables|/Script/ProjectW.MeshPlayerCharacter|SetcurrentBlockstunFrames (Variables|/Game/Gamemodes/FightingGamemodeBlueprint.FightingGamemodeBlueprint_C|Getplayer1Reference _asfighting_gamemode_blueprint) (Variables|Default|GethitboxBlockstunFrames))
          (Game|Damage|ApplyDamage (Variables|/Game/Gamemodes/FightingGamemodeBlueprint.FightingGamemodeBlueprint_C|Getplayer1Reference _asfighting_gamemode_blueprint) (Variables|Default|GethitboxDamage) 0 0))))))

(event EventBeginPlay)

(event Collision|EventActorBeginOverlap
  (params (OtherActor :type Actor%20Object%20Reference)))

(event EventTick
  (params (DeltaSeconds :type Float%20%28single-precision%29)))

(fn ConstructionScript)

(fn GetNewHitboxLocation
  (bind _self self)
  (bind _hitboxoffset (Variables|Default|GethitboxOffset))
  (bind _returnvalue (Components|GetOwner _self))
  (bind _returnvalue_2 (Transformation|GetActorLocation _returnvalue))
  (return (Math|Vector|MakeVector (+ (* (.x _hitboxoffset) (.x (Transformation|GetActorForwardVector _returnvalue))) (.x _returnvalue_2)) (.y _returnvalue_2) (+ (.z _hitboxoffset) (.z _returnvalue_2)))))